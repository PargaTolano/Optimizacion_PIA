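; WeaponClass is an FPS weapon Blueprint that tracks magazine and reserve ammo for shooting and reloading.
; Shoot spends a round and fires an event dispatcher unless Reloading, calling Reload on an empty magazine.
; Reload sets a hardcoded six-round magazine and decrements reserve by one when reserve covers the shortfall, otherwise moves the remainder in without the reload dispatcher.
; An empty reserve triggers the no-ammo sound dispatcher.
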(fn Shoot
  (if (not (Variables|Default|Getreloading?))
    (if (> (Variables|Default|Getcurr%20mag) 0)
      (Math|Integer|DecrementInt (Variables|Default|Getcurr%20mag)
        (:%20%20
          (Default|CallShootDispatcherWeaponClass)))
      (else
        (CallFunction|Reload)))))

(fn Reload
  (if (> (Variables|Default|Getcurr%20ammo) 0)
    (if (< (Variables|Default|Getcurr%20mag) (Variables|Default|Getmag%20capacity))
      (bind _output_get (Variables|Default|Setaux_reload (- (Variables|Default|Getmag%20capacity) (Variables|Default|Getcurr%20mag))))
      (if (<= _output_get (Variables|Default|Getcurr%20ammo))
        (Variables|Default|Setcurr%20mag 6)
        (Variables|Default|Setcurr%20ammo (- (Variables|Default|Getcurr%20ammo) 1))
        (Default|CallReloadDispatcherWeaponClass)
        (else
          (Variables|Default|Setcurr%20mag (Variables|Default|Getcurr%20ammo))
          (Variables|Default|Setcurr%20ammo 0))))
    (else
      (Default|CallNoAmmoSoundDispatcherWeaponClass))))